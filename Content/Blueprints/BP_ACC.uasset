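; BP_ACC is an intersection monitoring actor that logs when BP_Car actors cross its two trigger volumes.
; Entering ACCBoundary prints the car's name, the current time and a predicted time computed from a fixed distance divided by its vehicle movement forward speed.
; IntersectionBoundary prints name and time on entry and time on exit.
; All output is debug prints, with no control applied to the cars.
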(event `self.ACCBoundary.OnComponentBeginOverlap`
  (params (OverlappedComponent :type "PrimitiveComponent Object Reference") (OtherActor :type "Actor Object Reference") (OtherComp :type "PrimitiveComponent Object Reference") (OtherBodyIndex :type Integer) (bFromSweep :type Boolean) (SweepResult :type "HitResult Structure (by ref)"))
  (bind _returnvalue (`GameplayStatics.GetTimeSeconds`))
  (bind _asbp_car (cast `/Game/Blueprints/BP_Car` OtherActor))
  (set `self.EnterTime` _returnvalue)
  (`KismetSystemLibrary.PrintString` (`KismetSystemLibrary.GetDisplayName` _asbp_car))
  (`KismetSystemLibrary.PrintString` (`KismetStringLibrary.Conv_DoubleToString` _returnvalue))
  (`KismetSystemLibrary.PrintString` (`KismetStringLibrary.Conv_DoubleToString` (+ (`self.EnterTime`) (/ 3530.0 (`ChaosVehicleMovementComponent.GetForwardSpeed` (`WheeledVehiclePawn.VehicleMovementComponent` _asbp_car)))))))

(event `self.IntersectionBoundary.OnComponentBeginOverlap`
  (params (OverlappedComponent :type "PrimitiveComponent Object Reference") (OtherActor :type "Actor Object Reference") (OtherComp :type "PrimitiveComponent Object Reference") (OtherBodyIndex :type Integer) (bFromSweep :type Boolean) (SweepResult :type "HitResult Structure (by ref)"))
  (bind _asbp_car (cast `/Game/Blueprints/BP_Car` OtherActor))
  (`KismetSystemLibrary.PrintString` (`KismetSystemLibrary.GetDisplayName` _asbp_car))
  (`KismetSystemLibrary.PrintString` (`KismetStringLibrary.Conv_DoubleToString` (`GameplayStatics.GetTimeSeconds`))))

(event `self.IntersectionBoundary.OnComponentEndOverlap`
  (params (OverlappedComponent :type "PrimitiveComponent Object Reference") (OtherActor :type "Actor Object Reference") (OtherComp :type "PrimitiveComponent Object Reference") (OtherBodyIndex :type Integer))
  (cast `/Game/Blueprints/BP_Car` OtherActor)
  (`KismetSystemLibrary.PrintString` (`KismetStringLibrary.Conv_DoubleToString` (`GameplayStatics.GetTimeSeconds`))))

(fn `UserConstructionScript`)